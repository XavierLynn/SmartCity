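; BP_FloatPicker is an in-world slider that lets the player pick a float by looking at it and holding an input key.
; While the key is down, a shared BP_Trace, found or spawned after BeginPlay, traces and calls Action on any picker hit.
; Action stores the hit's collision UV X as LastFloat, which Tick maps to the Cube handle's position.
; The construction script applies the plane and slider materials.
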(event Custom|Action
  ;[1 1 1] Select only "X" position and write this to "Last Float". "Last Float" will use different BP's.
  (Variables|Default|SetLastFloat (.x (.UV (Class|GameplayStatics|FindCollisionUV (Variables|/Game/A_EzDraw/Blueprints/Components/BP_Trace.BP_Trace_C|GetLastHitResult (Variables|Default|GetTrace)))))))

(event EventBeginPlay
  ;[1 1 1] Create "Trace" BP if it doesn't do early.
  (Utilities|FlowControl|Delay 0.2)
  (bind _outactors (Actor|GetAllActorsOfClass "/Game/A_EzDraw/Blueprints/Components/BP_Trace.BP_Trace_C"))
  (Utilities|IsValid (Utilities|Array|Get(acopy) _outactors)
    (:Is%20Valid
      (Variables|Default|SetTrace (Utilities|Array|Get(acopy) _outactors)))
    (:Is%20Not%20Valid
      (bind _returnvalue (Game|SpawnActorfromClass "/Game/A_EzDraw/Blueprints/Components/BP_Trace.BP_Trace_C" (Math|Transform|MakeTransform "0, 0, 0" "0, 0, 0" "1,1,1") "Undefined" 0 0))
      (Variables|Default|SetTrace _returnvalue))))

(event EventTick
  (params (DeltaSeconds :type Float%20%28single-precision%29))
  (bind _trace (Variables|Default|GetTrace))
  ;[1 1 1] Wait "key down event". After trace line from player to camera forward vector. After cast result to "float picker" and call "Action" event.
  (Transformation|SetRelativeLocation (Variables|Default|GetCube) (Math|Vector|MakeVector (Math|Float|MapRangeClamped (Variables|Default|GetLastFloat) 0.0 1.0 -5e+01 5e+01) 0.0 0.0) false false)
  (if (Game|Player|IsInputKeyDown (Game|GetPlayerController 0) (Variables|Default|GetInput))
    (Default|Trace _trace)
    (if (Variables|/Game/A_EzDraw/Blueprints/Components/BP_Trace.BP_Trace_C|GetLastRetVal _trace)
      (bind _asbp_float_picker (Utilities|Casting|CastToBP_FloatPicker (.hitactor (Variables|/Game/A_EzDraw/Blueprints/Components/BP_Trace.BP_Trace_C|GetLastHitResult (Variables|Default|GetTrace)))))
      (CallFunction|Action _asbp_float_picker))))

(fn ConstructionScript
  (Rendering|Material|SetMaterial (Variables|Default|GetPlane) 0 (Variables|Default|GetMaterial))
  (Rendering|Material|SetMaterial (Variables|Default|GetCube) 0 (Variables|Default|GetSliderMaterial)))