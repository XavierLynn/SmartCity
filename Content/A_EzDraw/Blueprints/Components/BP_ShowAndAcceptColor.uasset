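; BP_ShowAndAcceptColor is a color preview Blueprint that shows the chosen RGB color and passes it to the drawing canvas.
; On BeginPlay it creates a dynamic instance of M_MasterColor and applies it to its Plane.
; Every tick it reads LastFloat from the R, G and B references, then writes that color to the material's RGBM parameter and the Canvas DrawColor, with alpha fixed at one.
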(event EventTick
  (params (DeltaSeconds :type Float%20%28single-precision%29))
  ;[1 1 1] Set Vector parameter in material instance every tick.
  (Rendering|Material|SetVectorParameterValue (Variables|Default|GetRGB) "RGBM" (Utilities|Struct|MakeLinearColor (Variables|/Game/A_EzDraw/Blueprints/BP_FloatPicker.BP_FloatPicker_C|GetLastFloat (Variables|Default|GetR)) (Variables|/Game/A_EzDraw/Blueprints/BP_FloatPicker.BP_FloatPicker_C|GetLastFloat (Variables|Default|GetG)) (Variables|/Game/A_EzDraw/Blueprints/BP_FloatPicker.BP_FloatPicker_C|GetLastFloat (Variables|Default|GetB)) 1.0) :!class /Script/Engine.MaterialInstanceDynamic)
  (Variables|/Game/A_EzDraw/Blueprints/BP_MainCanvas.BP_MainCanvas_C|SetDrawColor (Variables|Default|GetCanvas) (Utilities|Struct|MakeLinearColor (Variables|/Game/A_EzDraw/Blueprints/BP_FloatPicker.BP_FloatPicker_C|GetLastFloat (Variables|Default|GetR)) (Variables|/Game/A_EzDraw/Blueprints/BP_FloatPicker.BP_FloatPicker_C|GetLastFloat (Variables|Default|GetG)) (Variables|/Game/A_EzDraw/Blueprints/BP_FloatPicker.BP_FloatPicker_C|GetLastFloat (Variables|Default|GetB)) 1.0)))

(event EventBeginPlay
  ;[1 1 1] Create and accept dynamic material
  (bind _returnvalue (Rendering|Material|CreateDynamicMaterialInstance "/Game/A_EzDraw/Materials/Components/M_MasterColor.M_MasterColor" "None" :!class /Script/Engine.KismetMaterialLibrary))
  (bind _output_get (Variables|Default|SetRGB _returnvalue))
  (Rendering|Material|SetMaterial (Variables|Default|GetPlane) 0 _output_get))

(fn ConstructionScript)