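; BP_EditCanvas is the edit panel for a drawing canvas, applying the state of its picker and clicker controls to the Canvas.
; Every Tick it polls those controls, mapping the picker value to brush boldness and setting mask, draw mode and brush material from selected clickers.
; The brush uses the selected clicker's TurnOffMaterial.
; The clear clicker wipes the board with the draw or clear color, then switches itself off.
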(event EventTick
  (params (DeltaSeconds :type Float%20%28single-precision%29))
  (bind _canvas (Variables|Default|GetCanvas))
  (Utilities|FlowControl|Sequence
    (:then_0
      ;[1 1 1] Boldness
      (Variables|/Game/A_EzDraw/Blueprints/BP_MainCanvas.BP_MainCanvas_C|SetBoldness%20/%20Size (Variables|Default|GetCanvas) (Math|Float|MapRangeClamped (Variables|/Game/A_EzDraw/Blueprints/BP_FloatPicker.BP_FloatPicker_C|GetLastFloat (Variables|Default|GetBolndessPicker)) 0.0 1.0 1.0 128.0)))
    (:then_1
      ;[1 1 1] Select mask
      (for (_array_element _array_index) (Variables|Default|GetClickers_Masks)
        (if (Variables|/Game/A_EzDraw/Blueprints/BP_ClickButton.BP_ClickButton_C|GetSelected _array_element)
          (Variables|/Game/A_EzDraw/Blueprints/BP_MainCanvas.BP_MainCanvas_C|SetMask _canvas (Utilities|Array|Get(acopy) (Variables|Default|GetMasks) _array_index))
          (Default|UpdateMask _canvas))))
    (:then_2
      ;[1 1 1] Clear board
      (if (Variables|/Game/A_EzDraw/Blueprints/BP_ClickButton.BP_ClickButton_C|GetSelected (Variables|Default|GetClearClicker))
        (Default|ClearBoard (Variables|Default|GetCanvas) (select (Variables|Default|GetUseSelectedClearDrawColor?) (Variables|/Game/A_EzDraw/Blueprints/BP_MainCanvas.BP_MainCanvas_C|GetDrawColor (Variables|Default|GetCanvas)) (Variables|Default|GetClearColor)))
        (Default|TurnOn/Off (Variables|Default|GetClearClicker) false)))
    (:then_3
      ;[1 1 1] Select draw mode
      (for (_array_element_2 _array_index_2) (Variables|Default|GetClickers_drawtypes)
        (if (Variables|/Game/A_EzDraw/Blueprints/BP_ClickButton.BP_ClickButton_C|GetSelected _array_element_2)
          (Variables|/Game/A_EzDraw/Blueprints/BP_MainCanvas.BP_MainCanvas_C|SetMode (Variables|Default|GetCanvas) (Utilities|Select :Index _array_index_2 :Option%200 "NewEnumerator0" :Option%201 "NewEnumerator2" :Option%202 "NewEnumerator1")))))
    (:then_4
      ;[1 1 1] Select draw material
      (for _array_element_3 (Variables|Default|GetClickers_Materials)
        (if (Variables|/Game/A_EzDraw/Blueprints/BP_ClickButton.BP_ClickButton_C|GetSelected _array_element_3)
          (Variables|/Game/A_EzDraw/Blueprints/BP_MainCanvas.BP_MainCanvas_C|SetBrush (Variables|Default|GetCanvas) (Variables|/Game/A_EzDraw/Blueprints/BP_ClickButton.BP_ClickButton_C|GetTurnOffMaterial _array_element_3)))))))

(fn ConstructionScript)