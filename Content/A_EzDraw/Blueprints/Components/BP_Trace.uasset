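; BP_Trace is a helper Blueprint that line traces along the first player's camera view.
; Its Trace event casts a complex-collision ray from the camera manager's location along its forward vector, using configurable distance, channel and ignored actors.
; The success flag and hit result are cached in LastRetVal and LastHitResult, with debug drawing off.
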(event Custom|Trace
  (bind _returnvalue (Game|GetPlayerCameraManager 0))
  (bind _returnvalue_2 (Transformation|GetActorLocation _returnvalue))
  (bind (_outhit _returnvalue_3) (Collision|LineTraceByChannel _returnvalue_2 (+ _returnvalue_2 (* (Transformation|GetActorForwardVector _returnvalue) (Variables|Default|GetDistance))) (Variables|Default|GetTraceChannel) true (Variables|Default|GetTraceIgnoreActors) "None" false))
  (Variables|Default|SetLastRetVal _returnvalue_3)
  (Variables|Default|SetLastHitResult _outhit))

(fn ConstructionScript)