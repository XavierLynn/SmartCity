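; Clickable world button actor that switches between on and off materials and works like a radio button, turning off the buttons in its DisableOnClick list.
; After a short BeginPlay delay it finds or spawns a shared BP_Trace actor.
; Each button polls its input key on Tick, runs that trace while held, and calls Action on whichever BP_ClickButton is hit, so it repeats every held frame.
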(event Custom|Action
  ;[1 1 1] Turn on this button and turn off another selected
  (CallFunction|TurnOn/Off true)
  (for _array_element (Variables|Default|GetDisableOnClick)
    (CallFunction|TurnOn/Off _array_element false)))

(event Custom|TurnOn/Off
  (params (Selected :type Boolean))
  ;[1 1 1] Set Selected and needed material.
  (bind _output_get (Variables|Default|SetSelected Selected))
  (Rendering|Material|SetMaterial (Variables|Default|GetPlane) 0 (select _output_get (Variables|Default|GetTurnOnMaterial) (Variables|Default|GetTurnOffMaterial))))

(event EventBeginPlay
  ;[1 1 1] Create "Trace" BP, if in doesn't do early.
  (Utilities|FlowControl|Delay 0.2)
  (bind _outactors (Actor|GetAllActorsOfClass "/Game/A_EzDraw/Blueprints/Components/BP_Trace.BP_Trace_C"))
  (Utilities|IsValid (Utilities|Array|Get(acopy) _outactors)
    (:Is%20Valid
      (Variables|Default|SetTrace (Utilities|Array|Get(acopy) _outactors)))
    (:Is%20Not%20Valid
      (bind _returnvalue (Game|SpawnActorfromClass "/Game/A_EzDraw/Blueprints/Components/BP_Trace.BP_Trace_C" (Math|Transform|MakeTransform "0, 0, 0" "0, 0, 0" "1,1,1") "Undefined" 0 0))
      (Variables|Default|SetTrace _returnvalue))))

(event EventTick
  (params (DeltaSeconds :type Float%20%28single-precision%29))
  (bind _trace (Variables|Default|GetTrace))
  ;[1 1 1] Wait key down event and trace from "player" to "camera forward vector". If tracing hit to anything, try cast "hit result" to clicker.
  (if (Game|Player|IsInputKeyDown (Game|GetPlayerController 0) (Variables|Default|GetInput))
    (Default|Trace _trace)
    (if (Variables|/Game/A_EzDraw/Blueprints/Components/BP_Trace.BP_Trace_C|GetLastRetVal _trace)
      (bind _asbp_click_button (Utilities|Casting|CastToBP_ClickButton (.hitactor (Variables|/Game/A_EzDraw/Blueprints/Components/BP_Trace.BP_Trace_C|GetLastHitResult (Variables|Default|GetTrace)))))
      (CallFunction|Action _asbp_click_button))))

(fn ConstructionScript
  (Rendering|Material|SetMaterial (Variables|Default|GetPlane) 0 (Variables|Default|GetTurnOffMaterial)))