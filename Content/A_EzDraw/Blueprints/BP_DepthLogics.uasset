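; BP_DepthLogics maintains a depth buffer render target around the player character, fed by an orthographic scene capture.
; Each Tick it moves to the player's XY, snapped to capture pixel centers to keep texels aligned.
; It passes the normalized move as an offset to M_DepthCheckBuffer and draws that into RT_DepthBuffer.
; MPC_Depth publishes capture size and location, and ClearOnStart optionally wipes both render targets on BeginPlay.
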(event Custom|Move
  (bind _returnvalue (/ 1.0 512.0))
  (bind _returnvalue_2 (Game|GetPlayerCharacter 0))
  (bind _returnvalue_3 (Transformation|GetActorLocation))
  (bind _scenecapturecomponent2d (Variables|Default|GetSceneCaptureComponent2D))
  (bind _returnvalue_4 (Transformation|GetActorLocation _returnvalue_2))
  (bind _orthowidth (Variables|/Script/Engine.SceneCaptureComponent2D|GetOrthoWidth _scenecapturecomponent2d))
  (bind _returnvalue_5 (* _orthowidth _returnvalue))
  (bind _returnvalue_6 (|(((floor((Position/PixelWorldSize)))+0.500000)*PixelWorldSize) (.y _returnvalue_4) _returnvalue_5))
  (bind _returnvalue_7 (|(((floor((Position/PixelWorldSize)))+0.500000)*PixelWorldSize) (.x _returnvalue_4) _returnvalue_5))
  (bind _returnvalue_8 (Math|Vector|MakeVector _returnvalue_7 _returnvalue_6 0.0))
  (bind _returnvalue_9 (- _returnvalue_8 _returnvalue_3))
  (Utilities|IsValid _returnvalue_2
    (:Is%20Valid
      (bind _output_get (Variables|Default|SetMove2D (Math|Vector2D|MakeVector2D (.x _returnvalue_9) (.y _returnvalue_9))))
      (Transformation|AddActorWorldOffset (Math|Vector|MakeVector (.x _output_get) (.y _output_get) 0.0))
      (Rendering|Material|SetVectorParameterValue "/Game/A_EzDraw/Materials/CustomDepthBasedMaterials/MPC_Depth.MPC_Depth" "Locate" (Math|Conversions|ToLinearColor(Vector) (Transformation|GetActorLocation)) :!class /Script/Engine.KismetMaterialLibrary))
    (:Is%20Not%20Valid
      ;[1 1 1] Wait for character. If character doesn't spawned, do nothing
      (Utilities|FlowControl|Delay 0.2)
      (CallFunction|Move))))

(event EventBeginPlay
  (Rendering|Material|SetScalarParameterValue "/Game/A_EzDraw/Materials/CustomDepthBasedMaterials/MPC_Depth.MPC_Depth" "CaptureSize1f" (Variables|/Script/Engine.SceneCaptureComponent2D|GetOrthoWidth (Variables|Default|GetSceneCaptureComponent2D)) :!class /Script/Engine.KismetMaterialLibrary)
  (bind _returnvalue (Rendering|Material|CreateDynamicMaterialInstance "/Game/A_EzDraw/Materials/CustomDepthBasedMaterials/M_DepthCheckBuffer.M_DepthCheckBuffer" "None" :!class /Script/Engine.KismetMaterialLibrary))
  (Variables|Default|SetDM _returnvalue)
  (if (Variables|Default|GetClearOnStart?)
    (Rendering|ClearRenderTarget2D "/Game/A_EzDraw/Materials/CustomDepthBasedMaterials/RT_DepthCapture.RT_DepthCapture")
    (Rendering|ClearRenderTarget2D "/Game/A_EzDraw/Materials/CustomDepthBasedMaterials/RT_DepthBuffer.RT_DepthBuffer")))

(event EventTick
  (params (DeltaSeconds :type Float%20%28single-precision%29))
  (bind _scenecapturecomponent2d (Variables|Default|GetSceneCaptureComponent2D))
  (bind _move2d (Variables|Default|GetMove2D))
  (bind _orthowidth (Variables|/Script/Engine.SceneCaptureComponent2D|GetOrthoWidth _scenecapturecomponent2d))
  (bind _returnvalue (/ _move2d _orthowidth))
  (CallFunction|Move)
  (Rendering|Material|SetVectorParameterValue (Variables|Default|GetDM) "Offset" (Utilities|Struct|MakeLinearColor (.x _returnvalue) (.y _returnvalue) 0.0 1.0) :!class /Script/Engine.MaterialInstanceDynamic)
  (Rendering|DrawMaterialtoRenderTarget "/Game/A_EzDraw/Materials/CustomDepthBasedMaterials/RT_DepthBuffer.RT_DepthBuffer" (Variables|Default|GetDM)))

(fn ConstructionScript)