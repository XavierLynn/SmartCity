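; BP_StreamTo is an EzDraw actor that mirrors another canvas by showing that canvas's material on its own mesh.
; It copies the material from OriginalCanvas onto slot 0 of the Plane component on BeginPlay, on UpdateMask, and every Tick when EventTickUpdate is enabled.
; The construction script applies a configurable static mesh and physics simulation setting to Plane.
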(event Custom|UpdateMask
  (Rendering|Material|SetMaterial (Variables|Default|GetPlane) 0 (Variables|/Game/A_EzDraw/Blueprints/BP_MainCanvas.BP_MainCanvas_C|GetMATERIAL (Variables|Default|GetOriginalCanvas))))

(event EventBeginPlay
  (Rendering|Material|SetMaterial (Variables|Default|GetPlane) 0 (Variables|/Game/A_EzDraw/Blueprints/BP_MainCanvas.BP_MainCanvas_C|GetMATERIAL (Variables|Default|GetOriginalCanvas))))

(event EventTick
  (params (DeltaSeconds :type Float%20%28single-precision%29))
  (if (Variables|Default|GetEventTickUpdate?)
    (Rendering|Material|SetMaterial (Variables|Default|GetPlane) 0 (Variables|/Game/A_EzDraw/Blueprints/BP_MainCanvas.BP_MainCanvas_C|GetMATERIAL (Variables|Default|GetOriginalCanvas)))))

(fn ConstructionScript
  (bind _plane (Variables|Default|GetPlane))
  (Components|StaticMesh|SetStaticMesh _plane (Variables|Default|GetMesh))
  (Physics|SetSimulatePhysics _plane (Variables|Default|GetSimulatePhysics?)))